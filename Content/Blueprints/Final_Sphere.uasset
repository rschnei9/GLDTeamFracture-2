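; Final sphere actor that triggers an end sequence when the player character overlaps its box.
; On overlap it activates an InterpToMovement component and plays a timeline that drives the actor's scale.
; When the timeline finishes, the player camera fades to solid white over several seconds and holds there.
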(event `self.Box.OnComponentBeginOverlap`
  (params (OverlappedComponent :type "PrimitiveComponent Object Reference") (OtherActor :type "Actor Object Reference") (OtherComp :type "PrimitiveComponent Object Reference") (OtherBodyIndex :type Integer) (bFromSweep :type Boolean) (SweepResult :type "HitResult Structure (by ref)"))
  (bind _asbp_third_person_character (cast `/Game/ThirdPerson/Blueprints/BP_ThirdPersonCharacter` (`GameplayStatics.GetPlayerCharacter` 0)))
  (set `self.As BP Third Person Character` _asbp_third_person_character)
  (if (== OtherActor (`self.As BP Third Person Character`))
    (`ActorComponent.Activate` (`self.InterpToMovement`) false)
    (bind (_direction _scale) (`Timeline|Timeline`)
      (:`Update`
        (`self.SetActorScale3D` _scale))
      (:`Finished`
        (`PlayerCameraManager.StartCameraFade` (`GameplayStatics.GetPlayerCameraManager` 0) 0.0 1.0 5.0 (struct :`R` 1.0 :`G` 1.0 :`B` 1.0 :`A` 1.0) false true)))))

(fn `UserConstructionScript`)