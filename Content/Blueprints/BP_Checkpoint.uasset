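; BP_Checkpoint is a checkpoint actor that updates the player's respawn point when touched.
; On box overlap by the player character, it stores that character's current transform as SpawnTransform on BP_ThirdPersonGameMode, then calls RaiseFlag.
; RaiseFlag plays the T_Flag timeline, but its lerp is unconnected, so each update sets the Cube to a zero relative location.
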(event `RaiseFlag`
  ; Raise Flag
  (bind (_direction _flagtrack) (`Timeline|T_Flag`)
    (:`Update`
      (`SceneComponent.K2_SetRelativeLocation` (`self.Cube`) (0.0 0.0 0.0) false false))))

(event `self.Box.OnComponentBeginOverlap`
  (params (OverlappedComponent :type "PrimitiveComponent Object Reference") (OtherActor :type "Actor Object Reference") (OtherComp :type "PrimitiveComponent Object Reference") (OtherBodyIndex :type Integer) (bFromSweep :type Boolean) (SweepResult :type "HitResult Structure (by ref)"))
  (bind _returnvalue (`GameplayStatics.GetPlayerCharacter` 0))
  ; Set Spawn Point
  (if (== OtherActor _returnvalue)
    (cast `/Game/ThirdPerson/Blueprints/BP_ThirdPersonCharacter` OtherActor)
    (bind _asbp_third_person_game_mode (cast `/Game/ThirdPerson/Blueprints/BP_ThirdPersonGameMode` (`GameplayStatics.GetGameMode`)))
    (set `/Game/ThirdPerson/Blueprints/BP_ThirdPersonGameMode.Spawn Transform` (`self.GetTransform` _returnvalue) _asbp_third_person_game_mode)
    (`self.RaiseFlag`)))

(fn `UserConstructionScript`)